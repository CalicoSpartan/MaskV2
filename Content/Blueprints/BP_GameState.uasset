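; BP_GameState is a game state Blueprint that sets up the in-game HUD and feeds its kill feed.
; On BeginPlay it adds the main UI, then adds an alive widget above it if player 0's BP_FPSCharacter is in the playing state, storing that widget on the character.
; CallHUDUpdate triggers AddKillFeedMessage, which creates an entry from the current KillFeedMessage and appends it to the UI's vertical box.
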(event Custom|AddKillFeedMessage
  (bind _returnvalue (UserInterface|CreateWidget "/Game/UI/KillFeedEntry.KillFeedEntry_C" 0 (Utilities|Text|ToText(String) (Variables|Default|GetKillFeedMessage))))
  (bind _output_get (Variables|Default|SetEntry _returnvalue))
  (Class|VerticalBox|AddChildtoVerticalBox (Variables|/Game/UI/InGameUI.InGameUI_C|GetVerticalBox_0 (stale EventBeginPlay _output_get)) _output_get))

(event EventBeginPlay
  (Utilities|FlowControl|Sequence
    (:then_0
      (bind _returnvalue (UserInterface|CreateWidget "/Game/UI/InGameUI.InGameUI_C"))
      (bind _output_get (Variables|Default|SetUI _returnvalue))
      (UserInterface|Viewport|AddtoViewport _output_get 0))
    (:then_1
      (bind _asbp_fpscharacter (Utilities|Casting|CastToBP_FPSCharacter (Game|GetPlayerCharacter 0))
        (:then
          (if (Utilities|Enum|Equal(Enum) (Class|FPSCharacter|GetCurrentState _asbp_fpscharacter) "EPlayerPlaying")
            (bind _returnvalue_2 (UserInterface|CreateWidget "/Game/UI/AliveUI.AliveUI_C"))
            (bind _output_get_2 (Variables|Default|SetAliveUI _returnvalue_2))
            (bind _output_get_3 (Variables|/Game/Blueprints/BP_FPSCharacter.BP_FPSCharacter_C|SetAliveWidget _asbp_fpscharacter _output_get_2))
            (UserInterface|Viewport|AddtoViewport _output_get_3 1)))
        (:CastFailed
          (Development|PrintString "cast to bp_fpscharacter failed" true true "(R=0.000000,G=0.660000,B=1.000000,A=1.000000)" 1e+02))))))

(event EventTick
  (params (DeltaSeconds :type Float%20%28single-precision%29)))

(event EventCallHUDUpdate
  (CallFunction|AddKillFeedMessage))

(fn ConstructionScript)